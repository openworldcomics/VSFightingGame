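; Global controller for a two-player fighting game, running character selection, match start and both players' input.
; It spawns the camera and selection actors, swapping preview characters as each player's number changes.
; CreateFighter replaces these with chosen fighters, possessing Player 1 itself and Player 2 through a spawned second controller.
; It routes move, jump and crouch to both, toggles input for pause, and each Tick sets facing from Player 1's look-at yaw, negated for Player 2.
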(event `self.ReceiveBeginPlay`
  ;[1 1 1] Begin Default
  (`self.DisableInput` null)
  ;[1 1 1] SpawCamera ACtor
  (`|SpawnActorFromClass` "/Game/Fight_Game/Blueprints/BP_CameraMaster.BP_CameraMaster_C" (`KismetMathLibrary.MakeTransform` (1010.0 0.0 223.0) (struct :`Pitch` 24.0 :`Yaw` -180.0)) "Undefined" "OverrideRootScale")
  ;[1 1 1] Spawn SelecActors
  (bind _returnvalue (`|SpawnActorFromClass` "/Game/Fight_Game/Blueprints/BP_Select_Player01.BP_Select_Player01_C" (`self.PositionSelectPlayer01`) "Undefined" "OverrideRootScale"))
  (set `self.Select01` _returnvalue)
  (set `self.P01_SelectObjetRemove` _returnvalue)
  (bind _returnvalue_2 (`|SpawnActorFromClass` "/Game/Fight_Game/Blueprints/BP_Select_Player02.BP_Select_Player02_C" (`self.PositionSelectPlayer02`) "Undefined" "OverrideRootScale"))
  (set `self.Select02` _returnvalue_2)
  (set `self.P02_SelectObjetRemove` _returnvalue_2))

(event `self.ReceiveTick`
  (params (DeltaSeconds :type "Float (single-precision)"))
  (bind _player01 (`self.Player01`))
  (bind _player02 (`self.Player02`))
  (bind _returnvalue (`KismetMathLibrary.MakeRotator` (.roll (`self.K2_GetActorRotation` _player01)) (.pitch (`self.K2_GetActorRotation` _player01)) (.yaw (`KismetMathLibrary.FindLookAtRotation` (`self.K2_GetActorLocation` _player01) (`self.K2_GetActorLocation` _player02)))))
  (`|ExecutionSequence`
    (:`then_0`
      (if (`self.SelectGame`)
        ;[1 1 1] Player 01  - Look to P02
        (`self.K2_SetActorRotation` _player01 _returnvalue true)
        ;[1 1 1] Invert Face (Player 02)
        (`self.K2_SetActorRotation` _player02 (* _returnvalue -1.0) false)))))

(event `DefaultPlayer`
  ;[1 1 1] SelectPlayer - DefaultBegin
  (bind _returnvalue (`|SpawnActorFromClass` "/Game/Fight_Game/Players/Char01/Blueprints/BP_Char01.BP_Char01_C" (`self.PositionSelectPlayer01`) "Undefined" "OverrideRootScale"))
  (set `self.P01_SelectObjetRemove` _returnvalue)
  (bind _returnvalue_2 (`|SpawnActorFromClass` "/Game/Fight_Game/Players/Char01/Blueprints/BP_Char01.BP_Char01_C" (`self.PositionSelectPlayer02`) "Undefined" "OverrideRootScale"))
  (set `self.P02_SelectObjetRemove` _returnvalue_2))

(event `InputAxis|Player01_Right`
  (params (AxisValue :type "Float (single-precision)"))
  ;[1 1 1] Player 01 Right/Back
  (`Pawn.AddMovementInput` (`self.Player01`) (0.0 -1.0 0.0) AxisValue false))

(event `InputAxis|Player02_Right`
  (params (AxisValue :type "Float (single-precision)"))
  ;[1 1 1] Player 02 Right/Back
  (`Pawn.AddMovementInput` (`self.Player02`) (0.0 -1.0 0.0) AxisValue false))

(event `PausePlay`
  ;[1 1 1] Pause Controller
  (if (`self.PauseGame`)
    (`self.DisableInput` null)
    (`self.DisableInput` (`self.Playe2Controler`))
    (else
      (`self.EnableInput` null)
      (`self.EnableInput` (`self.Playe2Controler`)))))

(event `InputAxis|Player01_Back`
  (params (AxisValue :type "Float (single-precision)"))
  ;[1 1 1] Player 01 Right/Back
  (`Pawn.AddMovementInput` (`self.Player01`) (0.0 -1.0 0.0) AxisValue false))

(event `InputAxis|Player02_Back`
  (params (AxisValue :type "Float (single-precision)"))
  ;[1 1 1] Player 02 Right/Back
  (`Pawn.AddMovementInput` (`self.Player02`) (0.0 -1.0 0.0) AxisValue false))

(event `GetSelectPlayers02`
  (bind _p02_number (`self.P02_Number`))
  (bind _positionselectplayer02 (`self.PositionSelectPlayer02`))
  (bind _p02_selectobjetremove (`self.P02_SelectObjetRemove`))
  ;[1 1 1] Select Player - ViewCharacter P2
  (`|ExecutionSequence`
    (:`then_0`
      (`/Engine/EditorBlueprintResources/StandardMacros.DoOnce` false :!label _label
        (:`Completed`
          (switch `int` _p02_number
            (:`1`
              (`self.K2_DestroyActor` _p02_selectobjetremove)
              (set `self.Temp_P02Number` _p02_number)
              (bind _returnvalue (`|SpawnActorFromClass` "/Game/Fight_Game/Players/Char01/Blueprints/BP_Char01.BP_Char01_C" _positionselectplayer02 "Undefined" "OverrideRootScale"))
              (set `self.P02_SelectObjetRemove` _returnvalue))
            (:`2`
              (`self.K2_DestroyActor` _p02_selectobjetremove)
              (set `self.Temp_P02Number` _p02_number)
              (bind _returnvalue_2 (`|SpawnActorFromClass` "/Game/Fight_Game/Players/Char02/Blueprints/BP_Char02.BP_Char02_C" _positionselectplayer02 "Undefined" "OverrideRootScale"))
              (set `self.P02_SelectObjetRemove` _returnvalue_2))))))
    (:`then_1`
      (if (!= (`self.P02_Number`) (`self.Temp_P02Number`))
        (goto _label :!via `Reset`)))))

(event `SelectPlayer01`
  (bind _positionselectplayer01 (`self.PositionSelectPlayer01`))
  (bind _p01_number (`self.P01_Number`))
  (bind _p01_selectobjetremove (`self.P01_SelectObjetRemove`))
  ;[1 1 1] Select Player - ViewCharacter P01
  (`|ExecutionSequence`
    (:`then_0`
      (`/Engine/EditorBlueprintResources/StandardMacros.DoOnce` false :!label _label_2
        (:`Completed`
          (switch `int` _p01_number
            (:`1`
              (`self.K2_DestroyActor` _p01_selectobjetremove)
              (set `self.Temp_P01Number` _p01_number)
              (bind _returnvalue (`|SpawnActorFromClass` "/Game/Fight_Game/Players/Char01/Blueprints/BP_Char01.BP_Char01_C" _positionselectplayer01 "Undefined" "OverrideRootScale"))
              (set `self.P01_SelectObjetRemove` _returnvalue))
            (:`2`
              (`self.K2_DestroyActor` _p01_selectobjetremove)
              (set `self.Temp_P01Number` _p01_number)
              (bind _returnvalue_2 (`|SpawnActorFromClass` "/Game/Fight_Game/Players/Char02/Blueprints/BP_Char02.BP_Char02_C" _positionselectplayer01 "Undefined" "OverrideRootScale"))
              (set `self.P01_SelectObjetRemove` _returnvalue_2))))))
    (:`then_1`
      (if (!= (`self.P01_Number`) (`self.Temp_P01Number`))
        (goto _label_2 :!via `Reset`)))))

(event `InputAction|Player02_Jump`
  (params (Key :type "Key Structure" :default "AnyKey"))
  (bind _player02 (`self.Player02`))
  (bind _returnvalue (`Pawn.GetMovementComponent` _player02))
  ;[1 1 1] Player02 JUMP
  (:`Pressed`
    (bind _ascharacter (cast `Character` _player02))
    (if (`NavMovementComponent.IsFalling` _returnvalue)
      _
      (elif (not (`NavMovementComponent.IsCrouching` _returnvalue))
        (`Character.Jump` _ascharacter))))
  (:`Released`
    (`Character.StopJumping` _ascharacter)))

(event `InputAction|Player01_Jump`
  (params (Key :type "Key Structure" :default "AnyKey"))
  (bind _player01 (`self.Player01`))
  ;[1 1 1] Player 01 JUMP
  (:`Pressed`
    (bind _ascharacter (cast `Character` _player01))
    (if (not (`NavMovementComponent.IsFalling` (`Pawn.GetMovementComponent` _player01)))
      (`Character.Jump` _ascharacter)))
  (:`Released`
    (`Character.StopJumping` _ascharacter)))

(event `InputAction|Player01_crouch`
  (params (Key :type "Key Structure" :default "AnyKey"))
  (bind _player01 (`self.Player01`))
  (bind _returnvalue (`Pawn.GetMovementComponent` _player01))
  (bind _returnvalue_2 (`NavMovementComponent.IsCrouching` _returnvalue))
  ;[1 1 1] Player01 CROUCH
  (:`Pressed`
    (bind _ascharacter (cast `Character` _player01))
    (if (`NavMovementComponent.IsFalling` _returnvalue)
      _
      (elif (not _returnvalue_2)
        (`Character.Crouch` _ascharacter))))
  (:`Released`
    (if _returnvalue_2
      (`Character.UnCrouch` _ascharacter))))

(event `InputAction|Player02_crouch`
  (params (Key :type "Key Structure" :default "AnyKey"))
  (bind _player02 (`self.Player02`))
  (bind _returnvalue (`Pawn.GetMovementComponent` _player02))
  (bind _returnvalue_2 (`NavMovementComponent.IsCrouching` _returnvalue))
  ;[1 1 1] Player02 CROUCH
  (:`Pressed`
    (bind _ascharacter (cast `Character` _player02))
    (if (`NavMovementComponent.IsFalling` _returnvalue)
      _
      (elif (not _returnvalue_2)
        (`Character.Crouch` _ascharacter))))
  (:`Released`
    (if _returnvalue_2
      (`Character.UnCrouch` _ascharacter))))

(event `CreateFighter`
  ;[1 1 1] Start Player
  (`self.K2_DestroyActor` (`self.P02_SelectObjetRemove`))
  (`self.K2_DestroyActor` (`self.P01_SelectObjetRemove`))
  (bind _returnvalue (`|SpawnActorFromClass` "/Game/Fight_Game/Blueprints/BP_Player02_Controller.BP_Player02_Controller_C" (`self.PositionPlayer02`) "Undefined" "OverrideRootScale"))
  (set `self.Playe2Controler` _returnvalue)
  (`self.GetPlayer01`)
  (`self.GetPlayer02`)
  (set `self.SelectGame` true)
  (`self.EnableInput` null)
  (`self.EnableInput` (`self.Playe2Controler`))
  ;[1 1 1] Destroy Select_Actors
  (bind _outactors (`GameplayStatics.GetAllActorsOfClass` "/Game/Fight_Game/Blueprints/BP_Select_Player01.BP_Select_Player01_C"))
  (`self.K2_DestroyActor` _outactors)
  (bind _outactors_2 (`GameplayStatics.GetAllActorsOfClass` "/Game/Fight_Game/Blueprints/BP_Select_Player02.BP_Select_Player02_C"))
  (`self.K2_DestroyActor` _outactors_2))

(fn `GetPlayer01`
  (bind _player01 (`self.Player01`))
  ;[1 1 1] Same number for Fight Game Menu
  ; Function= "GameSelectMenu"
  (switch `int` (`self.P01_Number`)
    (:`1`
      (bind _returnvalue (`|SpawnActorFromClass` "/Game/Fight_Game/Players/Char01/Blueprints/BP_Char01.BP_Char01_C" (`self.PositionPlayer01`) "Undefined" "OverrideRootScale"))
      (set `self.Player01` _returnvalue)
      (`self.Possess` (`self.Player01`))
      (set `self.P01_Number` 0))
    (:`2`
      (bind _returnvalue_2 (`|SpawnActorFromClass` "/Game/Fight_Game/Players/Char02/Blueprints/BP_Char02.BP_Char02_C" (`self.PositionPlayer01`) "Undefined" "OverrideRootScale" _player01 _player01))
      (set `self.Player01` _returnvalue_2)
      (`self.Possess` (`self.Player01`))
      (set `self.P01_Number` 0))))

(fn `GetPlayer02`
  ;[1 1 1] Attection for this numbers (Menu)
  (switch `int` (`self.P02_Number`)
    (:`1`
      ;[1 1 1] Copy These Sequence for you New Character
      (bind _returnvalue (`|SpawnActorFromClass` "/Game/Fight_Game/Players/Char01/Blueprints/BP_Char01.BP_Char01_C" (`self.PositionPlayer02`) "Undefined" "OverrideRootScale"))
      (set `self.Player02` _returnvalue)
      (`self.Possess` (`self.Playe2Controler`) (`self.Player02`))
      (set `self.P02_Number` 0))
    (:`2`
      (bind _returnvalue_2 (`|SpawnActorFromClass` "/Game/Fight_Game/Players/Char02/Blueprints/BP_Char02.BP_Char02_C" (`self.PositionPlayer02`) "Undefined" "OverrideRootScale"))
      (set `self.Player02` _returnvalue_2)
      (`self.Possess` (`self.Playe2Controler`) (`self.Player02`))
      (set `self.P02_Number` 0))))

(fn `UserConstructionScript`)